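; GM_Room is the Game Mode for a multiplayer room lobby, tracking joined player controllers and launching the match.
; PostLogin pulls server name and player limit from GI_AllLevels, initializes each PC_Room, then rebroadcasts the player list to everyone.
; Map setting changes are pushed to every controller, as is the loading screen before a console ServerTravel to a hardcoded Test map.
; CallKickPlayer is an empty stub.
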(event `self.K2_PostLogin`
  (params (NewPlayer :type "PlayerController Object Reference"))
  ;[1 1 1] Update Info and Call Every Player Update
  (`/Engine/EditorBlueprintResources/ActorMacros.Switch Has Authority`
    (:`Authority`
      (`KismetArrayLibrary.Array_Add` (`self.AllPlayerControllers`) NewPlayer)
      (bind _asgi_all_levels (cast `/Game/BluePrints/AllLevels/GI_AllLevels` (`GameplayStatics.GetGameInstance`)))
      (set `self.ServerName` (`/Game/BluePrints/AllLevels/GI_AllLevels.ServerName` _asgi_all_levels))
      (set `self.MaxPlayers` (`/Game/BluePrints/AllLevels/GI_AllLevels.MaxPlayers` _asgi_all_levels))
      (bind _aspc_room (cast `/Game/BluePrints/Room/PC_Room` NewPlayer))
      (`/Game/BluePrints/Room/PC_Room.LoadInfo` _aspc_room)
      (`/Game/BluePrints/Room/PC_Room.ShowRoomMenu` _aspc_room (`self.ServerName`))
      (`/Game/BluePrints/Room/PC_Room.UpdateGameSettings` _aspc_room (`self.MapImage`) (`self.MapName`) (`self.GameTime`))
      (`self.EveryoneUpdate`))))

(event `EveryoneUpdate`
  (bind _allplayercontrollers (`self.AllPlayerControllers`))
  ;[1 1 1] Call Everyone to Update Info and UI
  (`KismetArrayLibrary.Array_Clear` (`self.PlayerInfos`))
  (for _array_element _allplayercontrollers
    (bind _aspc_room (cast `/Game/BluePrints/Room/PC_Room` _array_element))
    (`KismetArrayLibrary.Array_Add` (`self.PlayerInfos`) (`/Game/BluePrints/Room/PC_Room.PlayerInfo` _aspc_room)))
  (for _array_element_2 _allplayercontrollers
    (bind _aspc_room_2 (cast `/Game/BluePrints/Room/PC_Room` _array_element_2))
    (`/Game/BluePrints/Room/PC_Room.UpdateRoomInfo` _aspc_room_2 (`self.PlayerInfos`) (`self.MaxPlayers`))))

(event `ServerUpdateGameSettings`
  (params (MapImage :type "Texture2D Object Reference") (MapName :type Text) (MapTime :type Text) (MapID :type Integer))
  ;[1 1 1] Server Do Change Map Settings and Replicate to Clients
  (set `self.MapImage` MapImage)
  (set `self.MapName` MapName)
  (set `self.GameTime` MapTime)
  (set `self.MapID` MapID)
  (for _array_element (`self.AllPlayerControllers`)
    (bind _aspc_room (cast `/Game/BluePrints/Room/PC_Room` _array_element))
    (`/Game/BluePrints/Room/PC_Room.UpdateGameSettings` _aspc_room (`self.MapImage`) (`self.MapName`) (`self.GameTime`))))

(event `CallLaunchGame`
  ;[1 1 1] Server Call Everyone to Show Loading Screen and ServerTravel to Game Map
  (for _array_element (`self.AllPlayerControllers`)
    (bind _aspc_room (cast `/Game/BluePrints/Room/PC_Room` _array_element))
    (`/Game/BluePrints/Room/PC_Room.ShowLoadingScreen` _aspc_room))
  (switch `int` (`self.MapID`)
    (:`Default`
      (`KismetSystemLibrary.ExecuteConsoleCommand` "ServerTravel /Game/Maps/Test" (`GameplayStatics.GetPlayerController` 0)))))

(event `CallKickPlayer`
  (params (PlayerID :type Integer)))

(fn `UserConstructionScript`)