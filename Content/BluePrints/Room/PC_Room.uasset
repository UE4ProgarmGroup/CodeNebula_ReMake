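; Player controller for the multiplayer room lobby that shows the room menu and loading screen, and leaves the session when kicked.
; It loads saved player info, marks it as host or not ready, and asks GM_Room to update everyone.
; Chat goes out through GM_Room, while incoming messages, player lists and game settings feed into the menu widget.
; List and settings updates poll until that widget is valid.
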(event `ShowRoomMenu`
  (params (RoomName :type Text) (MaxPlayers :type Integer))
  ;[1 1 1] Set up and Display the Room Menu
  (set `self.bShowMouseCursor` true)
  (bind _returnvalue (`|CreateWidget` "/Game/UI/Room/RoomMenu.RoomMenu_C" null RoomName MaxPlayers))
  (bind _output_get (set `self.RoomMenuWB` _returnvalue))
  (`UserWidget.AddToViewport` _output_get 0)
  (`WidgetBlueprintLibrary.SetInputMode_UIOnlyEx` self _output_get))

(event `Kicked`
  ;[1 1 1] Kicked - Destroy Session when be Kicked
  (`NetGameInstance.LeaveRoom` (cast `/Game/BluePrints/AllLevels/GI_AllLevels` (`GameplayStatics.GetGameInstance`) :!pure true)))

(event `LoadInfo`
  ;[1 1 1] Load Player Info and Call EveryOne Sync Player Infos
  ;;[1 1 1] Load Player Info and Call Update Player List
  (`self.LoadGame`)
  (`self.CallUpdate` (`self.PlayerInfo`)))

(event `CallSendMessage`
  (params (Message :type Text))
  ;[1 1 1] Send and Receive Message
  ;;[1 1 1] CallSendMessage - Send Message
  (bind _asgm_room (cast `/Game/BluePrints/Room/GM_Room` (`GameplayStatics.GetGameMode`)))
  (`/Game/BluePrints/Room/GM_Room.SendMessage` _asgm_room (`.PlayerName_5_38EC61E243E4B80AEA882AB6BE1A026B` (break `/Game/BluePrints/AllLevels/PlayerInfo` (`self.PlayerInfo`))) Message))

(event `CallUpdate`
  (params (PlayerInfo :type "/Game/BluePrints/AllLevels/PlayerInfo Structure"))
  ;[1 1 1] Load Player Info and Call EveryOne Sync Player Infos
  ;;[1 1 1] Call Update Player List
  (set `self.PlayerInfo` PlayerInfo)
  (bind _asgm_room (cast `/Game/BluePrints/Room/GM_Room` (`GameplayStatics.GetGameMode`)))
  (`/Game/BluePrints/Room/GM_Room.CallEveryoneUpdate` _asgm_room))

(event `ShowLoadingScreen`
  ;[1 1 1] ShowLoadingScreen - Remove Room Menu and Display Loading Screen
  (`Widget.RemoveFromParent` (`self.RoomMenuWB`))
  (bind _returnvalue (`|CreateWidget` "/Game/UI/AllLevels/LoadingScreen.LoadingScreen_C" self))
  (`UserWidget.AddToViewport` _returnvalue 0))

(event `ReceiveMessage`
  (params (Sender :type Text) (Message :type Text))
  ;[1 1 1] Send and Receive Message
  ;;[1 1 1] ReceiveMessage - Show Received Message
  (`/Game/UI/Room/RoomMenu.AddMessage` (`self.RoomMenuWB`) Sender Message))

(event `UpdateRoomInfo`
  (params (PlayerInfos :type "Array of /Game/BluePrints/AllLevels/PlayerInfo Structure"))
  (bind _gamesettings (`/Game/UI/Room/RoomMenu.GameSettings` (`self.RoomMenuWB`)))
  ;[1 1 1] UpdateRoomInfo - Update UI
  (set `self.PlayerInfos` PlayerInfos)
  (`self.WaitFor` (`self.RoomMenuWB`))
  (`/Game/UI/Room/RoomMenu.UpdatePlayerWindow` (`self.RoomMenuWB`) (`self.PlayerInfos`))
  (`/Engine/EditorBlueprintResources/StandardMacros.IsValid` _gamesettings
    (:`Is Valid`
      (`/Game/UI/Room/GameSettings.UpdateKickList` _gamesettings (`self.PlayerInfos`)))))

(event `UpdateGameSettings`
  (params (MapImage :type "Texture2D Object Reference") (MapName :type Text) (GameTime :type Text))
  ;[1 1 1] UpdateGameSettings - Sync Game Settings
  (set `self.MapImage` MapImage)
  (set `self.MapName` MapName)
  (set `self.GameTime` GameTime)
  (`self.WaitFor` (`self.RoomMenuWB`))
  (`/Game/UI/Room/RoomMenu.UpdateGameSettings` (`self.RoomMenuWB`) (`self.MapImage`) (`self.MapName`) (`self.GameTime`)))

(fn `UserConstructionScript`)