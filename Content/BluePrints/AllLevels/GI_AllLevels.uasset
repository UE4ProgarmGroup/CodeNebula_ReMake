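; Game instance that manages menu display, game settings persistence and network error handling across all levels.
; ShowInitialMenu loads saved settings, applies the language culture, then opens the main menu if a player info save exists, otherwise the options menu.
; Main, host and options widgets are created once and reused, while the lobby menu is recreated on each call.
; Settings save to their own slot, and lost or timed-out connections trigger LeaveRoom.
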(event `ShowMainMenu`
  (bind _returnvalue (`GameplayStatics.GetPlayerController` 0))
  ;[1 1 1] ShowMainMenu - Show Main Menu and Enable Mouse Cursor
  (`/Engine/EditorBlueprintResources/StandardMacros.IsValid` (`self.MainMenuWB`)
    (:`Is Valid`
      _)
    (:`Is Not Valid`
      (bind _returnvalue_2 (`|CreateWidget` "/Game/UI/MainMenu/MainMenu.MainMenu_C" _returnvalue))
      (set `self.MainMenuWB` _returnvalue_2)))
  (`UserWidget.AddToViewport` (`self.MainMenuWB`) 0)
  (set `PlayerController.bShowMouseCursor` true _returnvalue))

(event `ShowInitialMenu`
  ;[1 1 1] ShowInitialMenu - Show Main Menu or Options Menu depends on Whether Save File Exists
  (`self.LoadGameSettings`)
  (`WidgetBlueprintLibrary.SetInputMode_UIOnlyEx` (`GameplayStatics.GetPlayerController` 0) null)
  (bind _returnvalue (`GameplayStatics.DoesSaveGameExist` (`self.PlayerInfoSave`)))
  (if _returnvalue
    (`self.ShowMainMenu`)
    (else
      (`self.ShowOptionsMenu`)
      (set `PlayerController.bShowMouseCursor` true (`GameplayStatics.GetPlayerController` 0)))))

(event `self.HandleNetworkError`
  (params (FailureType :type "ENetworkFailure Enum" :default "NetDriverAlreadyExists") (bIsServer :type Boolean))
  ;[1 1 1] Handle NetworkError
  (`KismetSystemLibrary.PrintString` (`|GetEnumeratorNameAsString` FailureType))
  (switch `ENetworkFailure` FailureType
    (:`ConnectionLost`
      _)
    (:`ConnectionTimeout`
      _))
  (`self.LeaveRoom`))

(event `ShowHostMenu`
  ;[1 1 1] ShowHostMenu - Show Host Game Menu
  (`/Engine/EditorBlueprintResources/StandardMacros.IsValid` (`self.HostMenuWB`)
    (:`Is Valid`
      _)
    (:`Is Not Valid`
      (bind _returnvalue (`|CreateWidget` "/Game/UI/MainMenu/HostMenu.HostMenu_C" (`GameplayStatics.GetPlayerController` 0)))
      (set `self.HostMenuWB` _returnvalue)))
  (`UserWidget.AddToViewport` (`self.HostMenuWB`) 0))

(event `LoadGameSettings`
  ;[1 1 1] Load Game Settings(If Exists
  (bind _returnvalue (`GameplayStatics.DoesSaveGameExist` (`self.GameSettingsSave`)))
  (if _returnvalue
    (bind _returnvalue_2 (`GameplayStatics.LoadGameFromSlot` (`self.GameSettingsSave`)))
    (bind _assg_game_settings (cast `/Game/BluePrints/AllLevels/SG_GameSettings` _returnvalue_2))
    (bind _output_get (set `self.GameSettings` (`/Game/BluePrints/AllLevels/SG_GameSettings.GameSettings` _assg_game_settings)))
    (`KismetInternationalizationLibrary.SetCurrentCulture` (`|GetEnumeratorNameAsString` (`.Language_22_A65951734A5BDB07050499BF68FC70B2` (break `/Game/BluePrints/AllLevels/GameSettings` _output_get))))))

(event `ShowLobbyMenu`
  ;[1 1 1] ShowLobbyMenu - Show Lobby Menu / Created each time when called
  (bind _returnvalue (`|CreateWidget` "/Game/UI/MainMenu/LobbyMenu.LobbyMenu_C" (`GameplayStatics.GetPlayerController` 0)))
  (`UserWidget.AddToViewport` _returnvalue 0))

(event `ShowOptionsMenu`
  ;[1 1 1] ShowOptionsMenu - Show Options Menu
  (`/Engine/EditorBlueprintResources/StandardMacros.IsValid` (`self.OptionsMenuWB`)
    (:`Is Valid`
      _)
    (:`Is Not Valid`
      (bind _returnvalue (`|CreateWidget` "/Game/UI/MainMenu/OptionsMenu.OptionsMenu_C" (`GameplayStatics.GetPlayerController` 0)))
      (set `self.OptionsMenuWB` _returnvalue)))
  (`UserWidget.AddToViewport` (`self.OptionsMenuWB`) 0))

(fn `Save Game Settings`
  (params (GameSettings :type "/Game/BluePrints/AllLevels/GameSettings Structure"))
  (bind _savegamesettingsref (`self.SaveGameSettingsRef`))
  (set `self.GameSettings` GameSettings)
  (`/Engine/EditorBlueprintResources/StandardMacros.IsValid` (`self.SaveGameSettingsRef`)
    (:`Is Valid`
      _)
    (:`Is Not Valid`
      (bind _returnvalue (`GameplayStatics.CreateSaveGameObject` "/Game/BluePrints/AllLevels/SG_GameSettings.SG_GameSettings_C"))
      (set `self.SaveGameSettingsRef` _returnvalue)))
  (set `/Game/BluePrints/AllLevels/SG_GameSettings.GameSettings` (`self.GameSettings`) _savegamesettingsref)
  (`GameplayStatics.SaveGameToSlot` _savegamesettingsref (`self.GameSettingsSave`)))