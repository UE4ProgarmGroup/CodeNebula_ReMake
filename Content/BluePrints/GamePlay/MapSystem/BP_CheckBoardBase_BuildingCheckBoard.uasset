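; Board tile holding a rotating planet with a random mesh and building count, which players manage or occupy.
; On the local player's turn, left-clicking an owned planet opens the main building menu; an unowned one marked ToBeOccupied is passed with the selected unit to the pawn's OccupyEve.
; RefreshWork re-totals works, material, energy and science from the building slots.
; SetColor swaps the tile base material by index.
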(event `self.ReceiveTick`
  (params (DeltaSeconds :type "Float (single-precision)"))
  (`SceneComponent.K2_AddLocalRotation` (`self.Planet`) (struct :`Pitch` 0.1) false false))

(event `RefreshWork`
  (`self.NewFunction_0`))

(event `self.Planet.OnClicked`
  (params (TouchedComponent :type "PrimitiveComponent Object Reference") (ButtonPressed :type "Key Structure"))
  (bind _asbp_pc_nebula (cast `/Game/BluePrints/GamePlay/Manager/BP_PC_Nebula` (`GameplayStatics.GetPlayerController` 0) :!pure true))
  (bind _asbp_pc_nebula_2 (cast `/Game/BluePrints/GamePlay/Manager/BP_PC_Nebula` (`GameplayStatics.GetPlayerController` 0) :!pure true))
  (if (`/Game/BluePrints/GamePlay/Manager/BP_PC_Nebula.GetTurn` _asbp_pc_nebula)
    (if (== ButtonPressed "LeftMouseButton")
      (if (== (`self.PlayerNum`) (`/Game/BluePrints/GamePlay/Manager/BP_PC_Nebula.Identity` _asbp_pc_nebula))
        (bind _foundwidgets (`WidgetBlueprintLibrary.GetAllWidgetsOfClass` "/Game/BluePrints/GamePlay/Widget/BuildingUI/W_MainBuidlingUI.W_MainBuidlingUI_C" false))
        (for _array_element _foundwidgets
          (`Widget.RemoveFromParent` _array_element))
        (bind _foundwidgets_2 (`WidgetBlueprintLibrary.GetAllWidgetsOfClass` "/Game/BluePrints/GamePlay/Widget/PlayerUI/MainUI.MainUI_C"))
        (`/Game/BluePrints/GamePlay/Widget/PlayerUI/MainUI.ShowMainBuildingMenu` (`|GetArrayItem` _foundwidgets_2) self)
        (else
          (`KismetSystemLibrary.PrintString` "NotMyPlanet")
          (if (`self.ToBeOccupied`)
            (bind _selectedunit (`/Game/BluePrints/GamePlay/Manager/BP_PC_Nebula.SelectedUnit` _asbp_pc_nebula_2)
              (:`then`
                (`/Game/BluePrints/GamePlay/Manager/BP_PP_Nebula.Occupy_Eve` (cast `/Game/BluePrints/GamePlay/Manager/BP_PP_Nebula` (`Controller.K2_GetPawn` _asbp_pc_nebula_2) :!pure true) _selectedunit self))
              (:`else`))))))))

(event `SetColor`
  (params (Index :type Integer))
  (`PrimitiveComponent.SetMaterial` (`self.BoardBase`) 0 (select `int` Index :`0` "/Game/Resource/Meterial/CheckBoard/CheckBoard_Inst.CheckBoard_Inst" :`1` "/Game/Resource/Meterial/CheckBoard/CheckBoard_Inst_1.CheckBoard_Inst_1" :`2` "/Game/Resource/Meterial/CheckBoard/CheckBoard_Inst_2.CheckBoard_Inst_2" :`3` "/Game/Resource/Meterial/CheckBoard/CheckBoard_Inst_3.CheckBoard_Inst_3" :`4` "/Game/Resource/Meterial/CheckBoard/CheckBoard_Inst_4.CheckBoard_Inst_4" :`5` "/Game/Resource/Meterial/CheckBoard/CheckBoard_Inst_5.CheckBoard_Inst_5" :`6` "/Game/Resource/Meterial/CheckBoard/CheckBoard_Inst_6.CheckBoard_Inst_6" :!type "MaterialInterface Object Reference")))

(fn `Init`
  (locals (NewLocalVar_0 :type "StaticMesh Object Reference"))
  (bind _planet (`self.Planet`))
  (bind _newlocalvar_0 (`local.NewLocalVar_0`))
  (set `local.NewLocalVar_0` (`KismetArrayLibrary.Array_Random` (`self.Mesh`)))
  (`StaticMeshComponent.SetStaticMesh` _planet _newlocalvar_0)
  (`PrimitiveComponent.SetMaterial` _planet 0 (`StaticMesh.GetMaterial` _newlocalvar_0 0))
  (set `self.BuildingNum` (`KismetMathLibrary.RandomIntegerInRange` 1 5)))

(fn `NewFunction_0`
  (set `self.Works` 0)
  (set `self.Material` 0)
  (set `self.Energy` 0)
  (set `self.SciencePoint` 0)
  (for _array_element (`self.BuildingSlot`)
    (`/Engine/EditorBlueprintResources/StandardMacros.IsValid` _array_element
      (:`Is Valid`
        (set `self.Works` (+ (`/Game/BluePrints/GamePlay/Player/Building/BP_BuildingBase.Choose` _array_element (`/Game/BluePrints/GamePlay/Player/Building/BP_BuildingBase.Works` _array_element)) (`self.Works`)))
        (set `self.Material` (+ (`/Game/BluePrints/GamePlay/Player/Building/BP_BuildingBase.Choose` _array_element (`/Game/BluePrints/GamePlay/Player/Building/BP_BuildingBase.Material` _array_element)) (`self.Material`)))
        (set `self.Energy` (+ (`/Game/BluePrints/GamePlay/Player/Building/BP_BuildingBase.Choose` _array_element (`/Game/BluePrints/GamePlay/Player/Building/BP_BuildingBase.Energy` _array_element)) (`self.Energy`)))
        (set `self.SciencePoint` (+ (`/Game/BluePrints/GamePlay/Player/Building/BP_BuildingBase.Choose` _array_element (`/Game/BluePrints/GamePlay/Player/Building/BP_BuildingBase.Science` _array_element)) (`self.SciencePoint`)))))))

(fn `UserConstructionScript`
  (`parent.UserConstructionScript`)
  (`self.Init`))