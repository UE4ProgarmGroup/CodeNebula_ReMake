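; Grid tile for unit movement on the Nebula board, tracking occupancy by box overlap and registering itself as the overlapping unit's board.
; On the server it caches nearby tiles as neighbours after a startup delay.
; Highlight functions recolour and flag tiles for moves to free neighbours, attacks, or jumps to free tiles near the owning player's buildings.
; Right-clicking a highlighted tile clears highlights and passes the selected unit's move or jump to the player pawn.
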(event `self.ReceiveBeginPlay`
  ;[1 1 1] 开始时获得相邻方格
  (`/Engine/EditorBlueprintResources/ActorMacros.Switch Has Authority`
    (:`Authority`
      (`KismetSystemLibrary.Delay` 5.0)
      (bind _outactors (`GameplayStatics.GetAllActorsOfClass` "BP_CheckBoardBase_MovingCheckBoard_C"))
      (for _array_element _outactors
        (if (<= (`KismetMathLibrary.VSize` (- (`self.K2_GetActorLocation` _array_element) (`self.K2_GetActorLocation`))) 150.0)
          (`KismetArrayLibrary.Array_Add` (`self.Neighbours`) _array_element))))))

(event `self.BoardBase.OnClicked`
  (params (TouchedComponent :type "PrimitiveComponent Object Reference") (ButtonPressed :type "Key Structure"))
  (bind _returnvalue (`GameplayStatics.GetPlayerController` 0))
  (bind _returnvalue_2 (`GameplayStatics.GetPlayerController` 0))
  (bind _returnvalue_3 (`GameplayStatics.GetPlayerController` 0))
  (bind _returnvalue_4 (`GameplayStatics.GetPlayerController` 0))
  (bind _asbp_pc_nebula (cast `/Game/BluePrints/GamePlay/Manager/BP_PC_Nebula` _returnvalue_4 :!pure true))
  (bind _asbp_pc_nebula_2 (cast `/Game/BluePrints/GamePlay/Manager/BP_PC_Nebula` _returnvalue_2 :!pure true))
  (bind _selectedunit (`/Game/BluePrints/GamePlay/Manager/BP_PC_Nebula.SelectedUnit` _asbp_pc_nebula))
  (bind _selectedunit_2 (`/Game/BluePrints/GamePlay/Manager/BP_PC_Nebula.SelectedUnit` _asbp_pc_nebula_2))
  (bind _board (`/Game/BluePrints/GamePlay/Player/Unit/BP_BaseUnit.Board` _selectedunit_2))
  ;[1 1 1] 右键单击简单移动
  (if (== ButtonPressed "RightMouseButton")
    (if (`self.MoveHighlight`)
      (bind _output_get (set `/Game/BluePrints/GamePlay/Manager/BP_PC_Nebula.MoveLocation` (`self.K2_GetActorLocation`) _asbp_pc_nebula_2))
      (`self.Resethighlight` _board)
      (set `PlayerController.bEnableClickEvents` false _returnvalue_3)
      (`/Game/BluePrints/GamePlay/Manager/BP_PP_Nebula.Move_Eve` (cast `/Game/BluePrints/GamePlay/Manager/BP_PP_Nebula` (`Controller.K2_GetPawn` _returnvalue_2) :!pure true) _output_get _selectedunit_2)
      (`KismetSystemLibrary.Delay` 0.5)
      (set `PlayerController.bEnableClickEvents` true _returnvalue_3)
      (`self.SetMoveHighlight` _board)
      (elif (`self.JumpHighlight`)
        (`KismetSystemLibrary.PrintString` "Hello")
        (bind _output_get_2 (set `/Game/BluePrints/GamePlay/Manager/BP_PC_Nebula.MoveLocation` (`self.K2_GetActorLocation`) _asbp_pc_nebula))
        (`self.Resethighlight` (`/Game/BluePrints/GamePlay/Player/Unit/BP_BaseUnit.Board` _selectedunit))
        (set `PlayerController.bEnableClickEvents` false _returnvalue)
        (`/Game/BluePrints/GamePlay/Manager/BP_PP_Nebula.Jump_Eve` (cast `/Game/BluePrints/GamePlay/Manager/BP_PP_Nebula` (`Controller.K2_GetPawn` _returnvalue_4) :!pure true) (`KismetMathLibrary.MakeVector` (.x _output_get_2) (.y _output_get_2) (+ (.z _output_get_2) 50.0)) _selectedunit)
        (`KismetSystemLibrary.Delay` 0.2)
        (set `PlayerController.bEnableClickEvents` true _returnvalue)))))

(event `self.Box.OnComponentBeginOverlap`
  (params (OverlappedComponent :type "PrimitiveComponent Object Reference") (OtherActor :type "Actor Object Reference") (OtherComp :type "PrimitiveComponent Object Reference") (OtherBodyIndex :type Integer) (bFromSweep :type Boolean) (SweepResult :type "HitResult Structure (by ref)"))
  ;[1 1 1] 设置单位所在的方格
  (bind _asbp_base_unit (cast `/Game/BluePrints/GamePlay/Player/Unit/BP_BaseUnit` OtherActor))
  (bind _output_get (set `/Game/BluePrints/GamePlay/Player/Unit/BP_BaseUnit.Board` self _asbp_base_unit))
  (`KismetSystemLibrary.PrintString` (`/Game/BluePrints/GamePlay/MapSystem/BP_CheckBoardBase_MovingCheckBoard.name` _output_get))
  (set `self.IsOccupied` true))

(event `self.Box.OnComponentEndOverlap`
  (params (OverlappedComponent :type "PrimitiveComponent Object Reference") (OtherActor :type "Actor Object Reference") (OtherComp :type "PrimitiveComponent Object Reference") (OtherBodyIndex :type Integer))
  (set `self.IsOccupied` false))

(fn `Resethighlight`
  (bind _outactors (`GameplayStatics.GetAllActorsOfClass` "BP_CheckBoardBase_MovingCheckBoard_C"))
  (for _array_element _outactors
    (`PrimitiveComponent.SetMaterial` (`/Game/BluePrints/GamePlay/MapSystem/BP_CheckBoardBase.BoardBase` _array_element) 0 "/Game/Resource/Meterial/CheckBoard/CheckBoard_Inst.CheckBoard_Inst")
    (set `/Game/BluePrints/GamePlay/MapSystem/BP_CheckBoardBase_MovingCheckBoard.MoveHighlight` false _array_element)
    (set `/Game/BluePrints/GamePlay/MapSystem/BP_CheckBoardBase_MovingCheckBoard.isEnermy` false _array_element)
    (set `/Game/BluePrints/GamePlay/MapSystem/BP_CheckBoardBase_MovingCheckBoard.JumpHighlight` false _array_element)
    (bind _outactors_2 (`GameplayStatics.GetAllActorsOfClass` "/Game/BluePrints/GamePlay/MapSystem/BP_CheckBoardBase_BuildingCheckBoard.BP_CheckBoardBase_BuildingCheckBoard_C"))
    (for _array_element_2 _outactors_2
      (set `/Game/BluePrints/GamePlay/MapSystem/BP_CheckBoardBase_BuildingCheckBoard.ToBeOccupied` false _array_element_2))))

(fn `SetEnermyHighlight`
  (`PrimitiveComponent.SetMaterial` (`self.BoardBase`) 0 "/Game/Resource/Meterial/CheckBoard/CheckBoard_Inst_Attack.CheckBoard_Inst_Attack")
  (set `self.isEnermy` true))

(fn `SetJumpHighlight`
  (params (In :type "/Game/BluePrints/GamePlay/Player/Unit/BP_BaseUnit Object Reference"))
  (bind _ownerpsid (`/Game/BluePrints/GamePlay/Player/Unit/BP_BaseUnit.OwnerPSId` In))
  (bind _playerarray (`GameStateBase.PlayerArray` (`GameplayStatics.GetGameState`)))
  (`KismetSystemLibrary.PrintString` (`KismetStringLibrary.Conv_IntToString` _ownerpsid))
  (for (_array_element _array_index) _playerarray
    (if (== (`PlayerState.PlayerId` _array_element) _ownerpsid)
      (break)))
  (bind _outactors (`GameplayStatics.GetAllActorsOfClass` "BP_CheckBoardBase_MovingCheckBoard_C"))
  (for _array_element_2 _outactors
    (if (not (`/Game/BluePrints/GamePlay/MapSystem/BP_CheckBoardBase.IsOccupied` _array_element_2))
      (for _array_element_3 (`/Game/BluePrints/GamePlay/Manager/BP_PS_Nebula.BuildingOwned` (cast `/Game/BluePrints/GamePlay/Manager/BP_PS_Nebula` (`|GetArrayItem` _playerarray _array_index) :!pure true))
        (if (< (`KismetMathLibrary.Vector_Distance` (`self.K2_GetActorLocation` _array_element_2) (`self.K2_GetActorLocation` _array_element_3)) 250.0)
          (`PrimitiveComponent.SetMaterial` (`/Game/BluePrints/GamePlay/MapSystem/BP_CheckBoardBase.BoardBase` _array_element_2) 0 "/Game/Resource/Meterial/CheckBoard/CheckBoard_Inst_Jump.CheckBoard_Inst_Jump")
          (set `/Game/BluePrints/GamePlay/MapSystem/BP_CheckBoardBase_MovingCheckBoard.JumpHighlight` true _array_element_2))))))

(fn `SetMoveHighlight`
  (for _array_element (`self.Neighbours`)
    (`KismetSystemLibrary.PrintString` (`KismetStringLibrary.Conv_VectorToString` (`self.K2_GetActorLocation` _array_element)))
    (if (not (`/Game/BluePrints/GamePlay/MapSystem/BP_CheckBoardBase.IsOccupied` _array_element))
      (`PrimitiveComponent.SetMaterial` (`/Game/BluePrints/GamePlay/MapSystem/BP_CheckBoardBase.BoardBase` _array_element) 0 "/Game/Resource/Meterial/CheckBoard/CheckBoard_Inst_Move.CheckBoard_Inst_Move")
      (set `/Game/BluePrints/GamePlay/MapSystem/BP_CheckBoardBase_MovingCheckBoard.MoveHighlight` true _array_element))))

(fn `UserConstructionScript`
  (`parent.UserConstructionScript`))