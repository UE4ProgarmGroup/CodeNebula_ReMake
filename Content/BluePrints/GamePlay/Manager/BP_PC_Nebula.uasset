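; Player controller for the turn-based Nebula game, handling turn flow, main UI setup and mothership spawning once a pawn is possessed.
; EndTurn advances the GameMode's player index, notifying all controllers to check for unitless defeat and wrapping into new rounds.
; Gaining a turn settles PlayerState buildings, advances unit production and adds science points to research.
; CallBuild and CallUnit spawn construction-site and production actors, registering them with PlayerState and their board.
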(event `TurnGetted`
  ;[1 1 1] TurnGetted  - Get Turn, Settle Own Buildings and Do Study
  (set `self.GetTurn` true)
  (bind _returnvalue (`|CreateWidget` "/Game/BluePrints/GamePlay/Widget/PlayerUI/ChildUI/OnYourTurn.OnYourTurn_C"))
  (`UserWidget.AddToViewport` _returnvalue 0)
  (`KismetSystemLibrary.PrintString` "Now My Turn.")
  (`self.BuildingSettlement` self)
  (`self.Study`))

(event `CheckDead`
  (bind _asbp_ps_nebula (cast `/Game/BluePrints/GamePlay/Manager/BP_PS_Nebula` (`self.PlayerState`)))
  (bind _returnvalue (`KismetArrayLibrary.Array_Length` (`/Game/BluePrints/GamePlay/Manager/BP_PS_Nebula.UnitsOwned` _asbp_ps_nebula)))
  (`KismetSystemLibrary.PrintString` (`KismetStringLibrary.Conv_IntToString` _returnvalue))
  (if (== _returnvalue 0)
    (`/Game/BluePrints/GamePlay/Manager/BP_GM_Nebula.Lost` (cast `/Game/BluePrints/GamePlay/Manager/BP_GM_Nebula` (`GameplayStatics.GetGameMode`) :!pure true) self)))

(event `TurnEnded`
  ;[1 1 1] Turn Ended - Show In Chat Window
  (`KismetSystemLibrary.PrintString` "Turn Ended.")
  (`self.CheckDead`))

(event `RoundEnded`
  ;[1 1 1] Switch Turn, Round - Client Handle Server Callback
  ;;[1 1 1] Round Ended - Show In Chat Window
  (`KismetSystemLibrary.PrintString` "Round Ended."))

(event `self.ReceiveBeginPlay`
  (bind (_language _render _illumination _particle _music _sound) (break `/Game/BluePrints/AllLevels/GameSettings` (`/Game/BluePrints/AllLevels/GI_AllLevels.GameSettings` (cast `/Game/BluePrints/AllLevels/GI_AllLevels` (`GameplayStatics.GetGameInstance`) :!pure true))))
  ;[1 1 1] 创建UI
  (`KismetSystemLibrary.Delay` 1.0)
  (if (`self.IsLocalPlayerController` self)
    (bind _returnvalue (`|CreateWidget` "/Game/BluePrints/GamePlay/Widget/PlayerUI/MainUI.MainUI_C" self))
    (`UserWidget.AddToViewport` _returnvalue 0)
    (set `self.MainUI` _returnvalue)
    (`WidgetBlueprintLibrary.SetInputMode_GameAndUIEx` self null)
    ;[1 1 1] 设置音乐，音效音量
    (`GameplayStatics.SetSoundMixClassOverride` null (`self.Audio`) (/ (`KismetMathLibrary.Conv_IntToDouble` _music) 100.0))
    (`GameplayStatics.SetSoundMixClassOverride` null (`self.Music`) (/ (`KismetMathLibrary.Conv_IntToDouble` _sound) 100.0))
    (`self.InitMainShip`)))

(event `BuildingSettlement`
  ;[1 1 1] BuildingSettlement - Settle Buildings
  (bind _asbp_ps_nebula (cast `/Game/BluePrints/GamePlay/Manager/BP_PS_Nebula` (`self.PlayerState`)))
  (`/Game/BluePrints/GamePlay/Manager/BP_PS_Nebula.Refresh` _asbp_ps_nebula)
  (for _array_element (`/Game/BluePrints/GamePlay/Manager/BP_PS_Nebula.BuildingOwned` _asbp_ps_nebula)
    (`/Game/BluePrints/GamePlay/Player/Building/BP_BuildingBase.EventActionOnTurn` _array_element))
  (for _array_element_2 (`/Game/BluePrints/GamePlay/Manager/BP_PS_Nebula.UnitProducing` _asbp_ps_nebula)
    (`/Game/BluePrints/GamePlay/Player/Unit/BP_ProducingUnit.Produce` _array_element_2))
  (bind _outactors (`GameplayStatics.GetAllActorsOfClass` "/Game/BluePrints/GamePlay/MapSystem/BP_CheckBoardBase_BuildingCheckBoard.BP_CheckBoardBase_BuildingCheckBoard_C"))
  (for _array_element_3 _outactors
    (`/Game/BluePrints/GamePlay/MapSystem/BP_CheckBoardBase_BuildingCheckBoard.RefreshWork` _array_element_3)))

(event `SwitchTurn`
  ;[1 1 1] Switch Turn, Round - Server Callback
  ;;[1 1 1] Switch Turn /  Each Player do Settlement and Into a New Round or Next Player get Turn - Called when Player call EndTurn
  (bind _asbp_gm_nebula (cast `/Game/BluePrints/GamePlay/Manager/BP_GM_Nebula` (`GameplayStatics.GetGameMode`)))
  (bind _currentplayerindex (`/Game/BluePrints/GamePlay/Manager/BP_GM_Nebula.CurrentPlayerIndex` _asbp_gm_nebula))
  (`/Engine/EditorBlueprintResources/StandardMacros.IncrementInt` _currentplayerindex
    (:`  `
      (bind _allplayercontrollers (`/Game/BluePrints/GamePlay/Manager/BP_GM_Nebula.AllPlayerControllers` _asbp_gm_nebula))
      (for _array_element _allplayercontrollers
        (bind _asbp_pc_nebula (cast `/Game/BluePrints/GamePlay/Manager/BP_PC_Nebula` _array_element))
        (`self.TurnEnded` _asbp_pc_nebula))
      (if (>= _currentplayerindex (`/Game/BluePrints/GamePlay/Manager/BP_GM_Nebula.PlayerNumber` _asbp_gm_nebula))
        (`self.SwitchRound`)
        (else
          (bind _asbp_pc_nebula_2 (cast `/Game/BluePrints/GamePlay/Manager/BP_PC_Nebula` (`|GetArrayItem` _allplayercontrollers _currentplayerindex)))
          (`self.TurnGetted` _asbp_pc_nebula_2))))))

(event `SwitchRound`
  ;[1 1 1] Switch Turn, Round - Server Callback
  ;;[1 1 1] Into a New Round / Each Player do Settlement and First Player get Turn
  (bind _asbp_gm_nebula (cast `/Game/BluePrints/GamePlay/Manager/BP_GM_Nebula` (`GameplayStatics.GetGameMode`)))
  (bind _allplayercontrollers (`/Game/BluePrints/GamePlay/Manager/BP_GM_Nebula.AllPlayerControllers` _asbp_gm_nebula))
  (for _array_element _allplayercontrollers
    (bind _asbp_pc_nebula (cast `/Game/BluePrints/GamePlay/Manager/BP_PC_Nebula` _array_element))
    (`self.RoundEnded` _asbp_pc_nebula))
  (set `/Game/BluePrints/GamePlay/Manager/BP_GM_Nebula.CurrentPlayerIndex` 0 _asbp_gm_nebula)
  (bind _asbp_pc_nebula_2 (cast `/Game/BluePrints/GamePlay/Manager/BP_PC_Nebula` (`|GetArrayItem` _allplayercontrollers)))
  (`self.TurnGetted` _asbp_pc_nebula_2))

(event `InitMainShip`
  (bind _returnvalue (`self.K2_GetPawn`))
  (bind _asbp_pp_nebula (cast `/Game/BluePrints/GamePlay/Manager/BP_PP_Nebula` _returnvalue :!pure true))
  (`/Engine/EditorBlueprintResources/StandardMacros.IsValid` (`self.K2_GetPawn`) :!label _label
    (:`Is Valid`
      (bind _output_get (set `/Game/BluePrints/GamePlay/Manager/BP_PP_Nebula.birthplace` (`self.K2_GetActorLocation` _returnvalue) _asbp_pp_nebula))
      (`/Game/BluePrints/GamePlay/Manager/BP_PP_Nebula.ShowSpawnFX` _asbp_pp_nebula _output_get)
      (`KismetSystemLibrary.Delay` 2.5)
      (bind _returnvalue_2 (`AIBlueprintHelperLibrary.SpawnAIFromClass` "/Game/BluePrints/GamePlay/Player/Unit/BP_BaseUnit_MotherShip.BP_BaseUnit_MotherShip_C" null (`KismetMathLibrary.MakeVector` (.x _output_get) (.y _output_get) (+ (.z _output_get) 100.0)) (`self.K2_GetActorRotation` _returnvalue) false null))
      (bind _asbp_base_unit_mother_ship (cast `/Game/BluePrints/GamePlay/Player/Unit/BP_BaseUnit_MotherShip` _returnvalue_2))
      (set `/Game/BluePrints/GamePlay/Player/Unit/BP_BaseUnit.Playernum` (`self.Identity`) _asbp_base_unit_mother_ship)
      (bind _asbp_ps_nebula (cast `/Game/BluePrints/GamePlay/Manager/BP_PS_Nebula` (`self.PlayerState`)))
      (`KismetArrayLibrary.Array_Add` (`/Game/BluePrints/GamePlay/Manager/BP_PS_Nebula.UnitsOwned` _asbp_ps_nebula) _asbp_base_unit_mother_ship))
    (:`Is Not Valid`
      (`KismetSystemLibrary.Delay` 0.2)
      (goto _label))))

(event `EndTurn`
  ;[1 1 1] Call Switch Turn - Client Call Server
  (if (`self.GetTurn`)
    (set `self.GetTurn` false)
    (`self.SwitchTurn`)
    (`KismetSystemLibrary.PrintString` "Call End Turn.")))

(event `CallBuild`
  (params (board :type "/Game/BluePrints/GamePlay/MapSystem/BP_CheckBoardBase_BuildingCheckBoard Object Reference") (ClassToBuild :type "/Game/BluePrints/GamePlay/Player/Building/BP_BuildingBase Class Reference") (BuildingSlotNum :type Integer))
  ;[1 1 1] 生产建筑工地
  (bind _returnvalue (`|SpawnActorFromClass` "/Game/BluePrints/GamePlay/Player/Building/BP_BuildingBase_Site.BP_BuildingBase_Site_C" (`self.GetTransform` board) "Undefined" "OverrideRootScale" self 1 ClassToBuild board BuildingSlotNum self null))
  (`KismetArrayLibrary.Array_Add` (`/Game/BluePrints/GamePlay/Manager/BP_PS_Nebula.BuildingOwned` (cast `/Game/BluePrints/GamePlay/Manager/BP_PS_Nebula` (`self.PlayerState`) :!pure true)) _returnvalue)
  (`KismetArrayLibrary.Array_Set` (`/Game/BluePrints/GamePlay/MapSystem/BP_CheckBoardBase_BuildingCheckBoard.BuildingSlot` board) BuildingSlotNum _returnvalue true))

(event `CallUnit`
  (params (Structure :type "/Game/BluePrints/GamePlay/Data/Structure/Stru_UnitProducing Structure") (ParentPanel :type "/Game/BluePrints/GamePlay/MapSystem/BP_CheckBoardBase_BuildingCheckBoard Object Reference"))
  ;[1 1 1] 生产单位生产Actor
  (bind _returnvalue (`|SpawnActorFromClass` "/Game/BluePrints/GamePlay/Player/Unit/BP_ProducingUnit.BP_ProducingUnit_C" (`self.GetTransform` ParentPanel) "Undefined" "OverrideRootScale" self ParentPanel Structure self null))
  (bind _output_get (set `self.LastProducedUnit` _returnvalue))
  (`KismetArrayLibrary.Array_Add` (`/Game/BluePrints/GamePlay/Manager/BP_PS_Nebula.UnitProducing` (cast `/Game/BluePrints/GamePlay/Manager/BP_PS_Nebula` (`self.PlayerState`) :!pure true)) _output_get)
  (`KismetArrayLibrary.Array_Add` (`/Game/BluePrints/GamePlay/MapSystem/BP_CheckBoardBase_BuildingCheckBoard.UnitsProducing` ParentPanel) _returnvalue))

(fn `ReFreshUnitBox`
  (params (PS :type "/Game/BluePrints/GamePlay/Manager/BP_PS_Nebula Object Reference"))
  (bind _foundwidgets (`WidgetBlueprintLibrary.GetAllWidgetsOfClass` "/Game/BluePrints/GamePlay/Widget/PlayerUI/MainUI.MainUI_C"))
  (bind _scrollbox_0 (`/Game/BluePrints/GamePlay/Widget/PlayerUI/ChildUI/W_RightBoard.ScrollBox_0` (`/Game/BluePrints/GamePlay/Widget/PlayerUI/MainUI.W_RightBoard` (cast `/Game/BluePrints/GamePlay/Widget/PlayerUI/MainUI` (`|GetArrayItem` _foundwidgets) :!pure true))))
  (for _array_element (`PanelWidget.GetAllChildren` _scrollbox_0)
    (bind _asw_unit (cast `/Game/BluePrints/GamePlay/Widget/PlayerUI/ChildUI/W_Unit` _array_element))
    (`Widget.RemoveFromParent` _asw_unit))
  (for _array_element_2 (`/Game/BluePrints/GamePlay/Manager/BP_PS_Nebula.UnitsOwned` PS)
    (bind _returnvalue (`|CreateWidget` "/Game/BluePrints/GamePlay/Widget/PlayerUI/ChildUI/W_Unit.W_Unit_C" null _array_element_2))
    (`PanelWidget.AddChild` _scrollbox_0 _returnvalue)))

(fn `Study`
  (locals (NewLocalVar_0 :type "/Game/BluePrints/GamePlay/Data/Structure/Stru_Skillstru Structure"))
  (bind _asbp_ps_nebula (cast `/Game/BluePrints/GamePlay/Manager/BP_PS_Nebula` (`self.PlayerState`) :!pure true))
  (bind _asbp_ps_nebula_2 (cast `/Game/BluePrints/GamePlay/Manager/BP_PS_Nebula` (`self.PlayerState`) :!pure true))
  (bind _skilldeveloping (`/Game/BluePrints/GamePlay/Manager/BP_PS_Nebula.SkillDeveloping` _asbp_ps_nebula))
  (bind _skill_skillarray (break `/Game/BluePrints/GamePlay/Data/Structure/Stru_TechList` (`/Game/BluePrints/GamePlay/Manager/BP_PS_Nebula.Skill` _asbp_ps_nebula)))
  (bind _skilldeveloping_2 (`/Game/BluePrints/GamePlay/Manager/BP_PS_Nebula.SkillDeveloping` _asbp_ps_nebula_2))
  (bind _skill_skillarray_2 (break `/Game/BluePrints/GamePlay/Data/Structure/Stru_TechList` (`/Game/BluePrints/GamePlay/Manager/BP_PS_Nebula.Skill` _asbp_ps_nebula_2)))
  (bind (_output_name _output_developed _output_schedule _output_scheduleneeded) (break `/Game/BluePrints/GamePlay/Data/Structure/Stru_Skillstru` (`|GetArrayItem` _skill_skillarray _skilldeveloping)))
  (bind (_output_name_2 _output_developed_2 _output_schedule_2 _output_scheduleneeded_2) (break `/Game/BluePrints/GamePlay/Data/Structure/Stru_Skillstru` (`|GetArrayItem` _skill_skillarray_2 _skilldeveloping_2)))
  (if (and (<= _skilldeveloping_2 19) (>= _skilldeveloping_2 0))
    (`KismetArrayLibrary.Array_Set` _skill_skillarray_2 _skilldeveloping_2 (make `/Game/BluePrints/GamePlay/Data/Structure/Stru_Skillstru` _output_name_2 _output_developed_2 (+ (`/Game/BluePrints/GamePlay/Manager/BP_PS_Nebula.SciencePoint` _asbp_ps_nebula_2) _output_schedule_2) _output_scheduleneeded_2))
    (if (> _output_schedule _output_scheduleneeded)
      (`KismetArrayLibrary.Array_Set` _skill_skillarray _skilldeveloping (make `/Game/BluePrints/GamePlay/Data/Structure/Stru_Skillstru` _output_name true _output_schedule _output_scheduleneeded)))))

(fn `UserConstructionScript`)