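; BP_PS_Nebula is a player state for a strategy game, tracking a player's resources, holdings and score.
; Call events forward costs to events that subtract Energy or Material (mineral) without checking the balance.
; Refresh resets per-round material income, maximum energy and science points, while CheckEnergy caps Energy at its maximum.
; SetScore only returns a weighted sum of owned and producing assets, lifetime gains, destroyed units and planets held.
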(event `CallCostEnergy`
  (params (Cost :type Integer))
  (`self.CostEnergy` Cost))

(event `CallCostMineral`
  (params (Cost :type Integer))
  (`self.CostMineral` Cost))

(event `CostEnergy`
  (params (Cost :type Integer))
  (set `self.Energy` (- (`self.Energy`) Cost)))

(event `CostMineral`
  (params (Cost :type Integer))
  (set `self.Material` (- (`self.Material`) Cost)))

(fn `CheckEnergy`
  (if (> (`self.Energy`) (`self.MaxEnergy`))
    (set `self.Energy` (`self.MaxEnergy`))))

(fn `Refresh`
  (set `self.MaterialEveryRound` 0)
  (set `self.MaxEnergy` 10)
  (set `self.SciencePoint` 0))

(fn `SetScore`
  (returns (ReturnValue :type Integer))
  (return (+ (+ (* (`KismetArrayLibrary.Array_Length` (`self.UnitsOwned`)) 5) (* (`KismetArrayLibrary.Array_Length` (`self.BuildingOwned`)) 5) (* (`KismetArrayLibrary.Array_Length` (`self.UnitProducing`)) 5)) (+ (`self.MaterialEverGain`) (`self.EnergyEverGain`) (`self.SciencePointEverGain`) (`self.WorksEverGain`)) (+ (* (`self.UnitDestoryed`) 3) (* (`self.PlanetEverHave`) 5)))))

(fn `UserConstructionScript`)