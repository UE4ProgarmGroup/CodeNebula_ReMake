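; BP_BuildingBase_3 is a player building that deals area damage to nearby units when its turn action runs.
; ActionOnturn scans all BP_BaseUnit actors and keeps those within a fixed radius of its board cell that are unowned or belong to another player.
; CallDamage then spawns a particle emitter above each target and applies fixed damage, crediting the owning PlayerController as damage causer.
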(event `CallDamage`
  (params (Actor :type "/Game/BluePrints/GamePlay/Player/Unit/BP_BaseUnit Object Reference"))
  (bind (_returnvalue_x _returnvalue_y _returnvalue_z) (`KismetMathLibrary.BreakVector` (`self.K2_GetActorLocation` Actor)))
  (`GameplayStatics.SpawnEmitterAtLocation` "/Game/Resource/Particle/Particle/Particle_Normal.Particle_Normal" (`KismetMathLibrary.MakeVector` 0.0 0.0 (+ _returnvalue_z 100.0)) (struct :`Pitch` -90.0))
  (`GameplayStatics.ApplyDamage` Actor 30.0 null (`self.PlayerController`)))

(fn `ActionOnturn`
  (`parent.ActionOnturn`)
  (`KismetArrayLibrary.Array_Clear` (`self.Out Actors`))
  (bind _outactors (`GameplayStatics.GetAllActorsOfClass` "/Game/BluePrints/GamePlay/Player/Unit/BP_BaseUnit.BP_BaseUnit_C"))
  (for _array_element _outactors
    (bind _playernum (`/Game/BluePrints/GamePlay/Player/Unit/BP_BaseUnit.Playernum` _array_element))
    (if (<= _playernum 0)
      (if (<= (`KismetMathLibrary.Vector_Distance` (`self.K2_GetActorLocation` _array_element) (`self.K2_GetActorLocation` (`self.CheckBoardIn`))) 230.0) :!label _label
        (`KismetArrayLibrary.Array_Add` (`self.Out Actors`) _array_element))
      (elif (!= (`|GetArrayItem` (`GameStateBase.PlayerArray` (`GameplayStatics.GetGameState`)) (- _playernum 1)) (`Controller.PlayerState` (`self.PlayerController`)))
        (goto _label))))
  (for _array_element_2 (`self.Out Actors`)
    (`self.CallDamage` _array_element_2)))

(fn `UserConstructionScript`
  (`parent.UserConstructionScript`))