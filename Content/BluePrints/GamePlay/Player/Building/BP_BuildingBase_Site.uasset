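; BP_BuildingBase_Site is a construction-site building that stands in for a building while it is being built over several turns.
; Each ActionOnturn calls the parent, then counts down BuildTurnsRemain.
; When the countdown ends, it spawns ClassToBuild in place with the same board, slot and controller, writes it into the checkboard's BuildingSlot, swaps itself for it in the player state's BuildingOwned list, and destroys itself.
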(fn `ActionOnturn`
  (bind _checkboardin (`self.CheckBoardIn`))
  (bind _playercontroller (`self.PlayerController`))
  (bind _buildingowned (`/Game/BluePrints/GamePlay/Manager/BP_PS_Nebula.BuildingOwned` (cast `/Game/BluePrints/GamePlay/Manager/BP_PS_Nebula` (`Controller.PlayerState` (`self.PlayerController`)) :!pure true)))
  (`parent.ActionOnturn`)
  (if (> (`self.BuildTurnsRemain`) 1)
    (`/Engine/EditorBlueprintResources/StandardMacros.DecrementInt` (`self.BuildTurnsRemain`))
    (else
      (bind _returnvalue (`|SpawnActorFromClass` (`self.ClassToBuild`) (`self.GetTransform`) "Undefined" "OverrideRootScale" _playercontroller _checkboardin (`self.BuildingSlotNum`) _playercontroller null))
      (`KismetArrayLibrary.Array_Set` (`/Game/BluePrints/GamePlay/MapSystem/BP_CheckBoardBase_BuildingCheckBoard.BuildingSlot` (cast `/Game/BluePrints/GamePlay/MapSystem/BP_CheckBoardBase_BuildingCheckBoard` _checkboardin :!pure true)) (`self.BuildingSlotNum`) _returnvalue true)
      (`KismetArrayLibrary.Array_RemoveItem` _buildingowned self)
      (`self.K2_DestroyActor`)
      (`KismetArrayLibrary.Array_Add` _buildingowned _returnvalue))))

(fn `UserConstructionScript`
  (`parent.UserConstructionScript`))