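; BP_ProducingUnit is an in-progress unit production order on a board tile that turns into a finished unit.
; Each Produce call subtracts the tile's Works from the remaining Works.
; Once that drops below zero, a sphere trace gathers unoccupied neighboring MovingCheckBoard tiles, printing a message if none exist.
; Otherwise it spawns UnitClass on a random one, flags a separately randomized pick as occupied, and destroys itself.
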(fn `Produce`
  (bind _outitem (`KismetArrayLibrary.Array_Random` (`self.CheckBoardCanBeUsed`)))
  ;[1 1 1] 生产信息
  (bind _output_get (set `self.Works` (- (`self.Works`) (`/Game/BluePrints/GamePlay/MapSystem/BP_CheckBoardBase_BuildingCheckBoard.Works` (`self.CheckBoardIn`)))))
  (if (< _output_get 0)
    ;[1 1 1] 判断生产地格周围地格占据情况
    (`KismetArrayLibrary.Array_Clear` (`self.CheckBoardCanBeUsed`))
    (bind _outhits (`KismetSystemLibrary.SphereTraceMulti` (`self.K2_GetActorLocation` (`self.CheckBoardIn`)) (0.0 0.0 0.0) 100.0 "TraceTypeQuery1"))
    (for _array_element _outhits
      (bind _asbp_check_board_base_moving_check_board (cast `/Game/BluePrints/GamePlay/MapSystem/BP_CheckBoardBase_MovingCheckBoard` (`.HitActor` (`GameplayStatics.BreakHitResult` _array_element))))
      (if (not (`/Game/BluePrints/GamePlay/MapSystem/BP_CheckBoardBase.IsOccupied` _asbp_check_board_base_moving_check_board))
        (`KismetArrayLibrary.Array_Add` (`self.CheckBoardCanBeUsed`) _asbp_check_board_base_moving_check_board)))
    ;[1 1 1] 生产单位
    (if (== 0 (`KismetArrayLibrary.Array_Length` (`self.CheckBoardCanBeUsed`)))
      (`KismetSystemLibrary.PrintString` "There Is No Place To Spawn new Unit")
      (else
        (`|SpawnActorFromClass` (`self.UnitClass`) (`self.GetTransform` _outitem) "Undefined" "OverrideRootScale" null null)
        (set `/Game/BluePrints/GamePlay/MapSystem/BP_CheckBoardBase.IsOccupied` true _outitem)
        (`self.K2_DestroyActor`)))))

(fn `UserConstructionScript`)