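; Base unit for a space strategy game that can move, portal-jump, attack and occupy planets.
; Action events play Niagara effects, disabling click input during timed ones; attacks use ray or missile by AttackMethod, and occupation accumulates per player until capture.
; Clicking an enemy unit requests an attack through the player pawn, while damage handles death and kill credit.
; The construction script applies the owner's tiered skills to health, damage and action costs.
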(event `self.ReceiveBeginPlay`
  ;[1 1 1] 控件赋值
  (bind _asw_unit_ui_choose (cast `/Game/BluePrints/GamePlay/Widget/ControllerUI/W_UnitUI_choose` (`WidgetComponent.GetWidget` (`self.Widget`))))
  (set `/Game/BluePrints/GamePlay/Widget/ControllerUI/W_UnitUI_choose.UnitContains` self _asw_unit_ui_choose))

(event `Move_Multi`
  (params (location :type "Vector Structure (by ref)"))
  ;[1 1 1] 移动
  (`AIBlueprintHelperLibrary.SimpleMoveToLocation` (`AIBlueprintHelperLibrary.GetAIController` self) location))

(event `Jump_Multi`
  (params (NewLocation :type "Vector Structure"))
  ;[1 1 1] 跃迁
  (`NiagaraFunctionLibrary.SpawnSystemAtLocation` "/Game/Resource/Particle/Niagara/Niagara/Portal_leave.Portal_leave" (`KismetMathLibrary.MakeVector` (.x (`self.K2_GetActorLocation` self)) (.y (`self.K2_GetActorLocation` self)) (- (.z (`self.K2_GetActorLocation` self)) 50.0)) (struct) (0.1 0.1 0.1))
  (set `PlayerController.bEnableClickEvents` false (`GameplayStatics.GetPlayerController` 0))
  (`NiagaraFunctionLibrary.SpawnSystemAtLocation` "/Game/Resource/Particle/Niagara/Niagara/Portal_Arrive.Portal_Arrive" (`KismetMathLibrary.MakeVector` (.x NewLocation) (.y NewLocation) (- (.z NewLocation) 50.0)) (struct) (0.2 0.2 0.2))
  (`ActorComponent.Activate` (`self.portal`) false)
  (`KismetSystemLibrary.Delay` 3.0)
  (`self.K2_SetActorLocation` self NewLocation false false)
  (set `PlayerController.bEnableClickEvents` true (`GameplayStatics.GetPlayerController` 0)))

(event `Attack_Multi`
  (params (DamagedActor :type "/Game/BluePrints/GamePlay/Player/Unit/BP_BaseUnit Object Reference"))
  (bind _returnvalue (`self.K2_GetActorLocation` DamagedActor))
  (bind _ray (`self.Ray`))
  (bind _missile (`self.Missile`))
  (bind _asbp_pc_nebula (cast `/Game/BluePrints/GamePlay/Manager/BP_PC_Nebula` (`GameplayStatics.GetPlayerController` 0) :!pure true))
  (bind _returnvalue_location (`KismetMathLibrary.BreakTransform` (`KismetMathLibrary.ConvertTransformToRelative` (`self.GetTransform` self) (`self.GetTransform` DamagedActor))))
  ;[1 1 1] 攻击：Attack Method 变量用于决定攻击方式
  (`self.K2_SetActorRotation` (`KismetMathLibrary.FindLookAtRotation` (`self.K2_GetActorLocation` self) _returnvalue))
  (switch `int` (`self.AttackMethod`)
    (:`0`
      (`NiagaraComponent.SetVariableVec3` _ray "EnermyTarget" _returnvalue)
      (`ActorComponent.Activate` _ray false)
      (`ActorComponent.Activate` (`self.lazer`) false))
    (:`1`
      (`NiagaraComponent.SetVariableVec3` _missile "Target" (`KismetMathLibrary.MakeVector` (.x _returnvalue_location) (.y _returnvalue_location) (- (.z _returnvalue_location) 80.0)))
      (`ActorComponent.Activate` _missile false)
      (`ActorComponent.Activate` (`self.missiles`) false)))
  (set `PlayerController.bEnableClickEvents` false _asbp_pc_nebula)
  (`KismetSystemLibrary.Delay` 1.0)
  (`GameplayStatics.ApplyDamage` DamagedActor (`self.Damage`) null (`|GetArrayItem` (`GameStateBase.PlayerArray` (`GameplayStatics.GetGameState`)) (`self.Playernum`)))
  (set `PlayerController.bEnableClickEvents` true _asbp_pc_nebula))

(event `Occupy_Muilti`
  (params (Planet :type "/Game/BluePrints/GamePlay/MapSystem/BP_CheckBoardBase_BuildingCheckBoard Object Reference"))
  (bind _playernum (`self.Playernum`))
  (bind _playeroccupation (`/Game/BluePrints/GamePlay/MapSystem/BP_CheckBoardBase_BuildingCheckBoard.PlayerOccupation` Planet))
  (bind _returnvalue (- (`self.Playernum`) 1))
  (bind _returnvalue_2 (+ (`|GetArrayItem` _playeroccupation _returnvalue) (`self.OccuPower`)))
  ;[1 1 1] 占领星球
  (`KismetArrayLibrary.Array_Set` _playeroccupation _returnvalue _returnvalue_2)
  (if (>= _returnvalue_2 10)
    (`KismetArrayLibrary.Array_Clear` _playeroccupation)
    (set `/Game/BluePrints/GamePlay/MapSystem/BP_CheckBoardBase_BuildingCheckBoard.PlayerNum` _playernum Planet)
    (`/Game/BluePrints/GamePlay/MapSystem/BP_CheckBoardBase_BuildingCheckBoard.SetColor` Planet _playernum)
    (`KismetArrayLibrary.Array_Clear` (`/Game/BluePrints/GamePlay/MapSystem/BP_CheckBoardBase_BuildingCheckBoard.BuildingSlot` Planet))
    (set `PlayerController.bEnableClickEvents` false (`GameplayStatics.GetPlayerController` 0))
    (`NiagaraFunctionLibrary.SpawnSystemAtLocation` "/Game/Resource/Particle/Niagara/Niagara/Occupy.Occupy" (`self.K2_GetActorLocation` Planet) (struct) (0.1 0.1 0.1))
    (`/Engine/EditorBlueprintResources/StandardMacros.IncrementInt` (`/Game/BluePrints/GamePlay/Manager/BP_PS_Nebula.PlanetEverHave` (cast `/Game/BluePrints/GamePlay/Manager/BP_PS_Nebula` (`|GetArrayItem` (`GameStateBase.PlayerArray` (`GameplayStatics.GetGameState`)) (`self.Playernum`)) :!pure true))
      (:`  `
        (`ActorComponent.Activate` (`self.occupy`) false)
        (`KismetSystemLibrary.Delay` 2.0)
        (set `PlayerController.bEnableClickEvents` true (`GameplayStatics.GetPlayerController` 0))))))

(event `self.CapsuleComponent.OnClicked`
  (params (TouchedComponent :type "PrimitiveComponent Object Reference") (ButtonPressed :type "Key Structure"))
  (bind _returnvalue (`GameplayStatics.GetPlayerController` 0))
  ;[1 1 1] 右键单击被攻击
  (if (== ButtonPressed "LeftMouseButton")
    (if (`/Game/BluePrints/GamePlay/MapSystem/BP_CheckBoardBase_MovingCheckBoard.isEnermy` (`self.Board`))
      (`/Game/BluePrints/GamePlay/Manager/BP_PP_Nebula.Attack_Eve` (cast `/Game/BluePrints/GamePlay/Manager/BP_PP_Nebula` (`Controller.K2_GetPawn` _returnvalue) :!pure true) (`/Game/BluePrints/GamePlay/Manager/BP_PC_Nebula.SelectedUnit` (cast `/Game/BluePrints/GamePlay/Manager/BP_PC_Nebula` _returnvalue :!pure true)) self))))

(event `self.ReceiveAnyDamage`
  (params (Damage :type "Float (single-precision)") (DamageType :type "DamageType Object Reference") (InstigatedBy :type "Controller Object Reference") (DamageCauser :type "Actor Object Reference"))
  ;[1 1 1] 被攻击时掉血
  (bind _output_get (set `self.Health` (- (`self.Health`) Damage)))
  (if (<= _output_get 0.0)
    (`ActorComponent.Activate` (`self.Explosion`) false)
    (`NiagaraFunctionLibrary.SpawnSystemAtLocation` "/Game/Resource/Particle/Niagara/Niagara/Boom.Boom" (`self.K2_GetActorLocation` self) (struct) (0.5 0.5 0.5))
    (`SceneComponent.SetVisibility` (`self.Mesh`) false false)
    (`/Engine/EditorBlueprintResources/StandardMacros.IncrementInt` (`/Game/BluePrints/GamePlay/Manager/BP_PS_Nebula.UnitDestoryed` (cast `/Game/BluePrints/GamePlay/Manager/BP_PS_Nebula` DamageCauser :!pure true))
      (:`  `
        (`KismetSystemLibrary.Delay` 2.0)
        (`self.K2_DestroyActor`)))))

(fn `UserConstructionScript`
  (bind _playernum (`self.Playernum`))
  (bind _skill_skillarray (break `/Game/BluePrints/GamePlay/Data/Structure/Stru_TechList` (`/Game/BluePrints/GamePlay/Manager/BP_PS_Nebula.Skill` (cast `/Game/BluePrints/GamePlay/Manager/BP_PS_Nebula` (`|GetArrayItem` (`GameStateBase.PlayerArray` (`GameplayStatics.GetGameState`)) (- _playernum 1)) :!pure true))))
  (bind (_output_name _output_developed) (break `/Game/BluePrints/GamePlay/Data/Structure/Stru_Skillstru` (`|GetArrayItem` _skill_skillarray 9)))
  (bind (_output_name_2 _output_developed_2) (break `/Game/BluePrints/GamePlay/Data/Structure/Stru_Skillstru` (`|GetArrayItem` _skill_skillarray 14)))
  (bind (_output_name_3 _output_developed_3) (break `/Game/BluePrints/GamePlay/Data/Structure/Stru_Skillstru` (`|GetArrayItem` _skill_skillarray 7)))
  (bind (_output_name_4 _output_developed_4) (break `/Game/BluePrints/GamePlay/Data/Structure/Stru_Skillstru` (`|GetArrayItem` _skill_skillarray 5)))
  (bind (_output_name_5 _output_developed_5) (break `/Game/BluePrints/GamePlay/Data/Structure/Stru_Skillstru` (`|GetArrayItem` _skill_skillarray 10)))
  (bind (_output_name_6 _output_developed_6) (break `/Game/BluePrints/GamePlay/Data/Structure/Stru_Skillstru` (`|GetArrayItem` _skill_skillarray 12)))
  (bind (_output_name_7 _output_developed_7) (break `/Game/BluePrints/GamePlay/Data/Structure/Stru_Skillstru` (`|GetArrayItem` _skill_skillarray)))
  (bind (_output_name_8 _output_developed_8) (break `/Game/BluePrints/GamePlay/Data/Structure/Stru_Skillstru` (`|GetArrayItem` _skill_skillarray 2)))
  (bind (_output_name_9 _output_developed_9) (break `/Game/BluePrints/GamePlay/Data/Structure/Stru_Skillstru` (`|GetArrayItem` _skill_skillarray 4)))
  (if (!= _playernum 0)
    (if _output_developed_4
      (if _output_developed_3
        (if _output_developed
          (set `self.MaxHealth` (* (`self.MaxHealth`) 2.0))
          (else
            (set `self.MaxHealth` (* (`self.MaxHealth`) 1.5))))
        (else
          (set `self.MaxHealth` (* (`self.MaxHealth`) 1.2)))))
    (set `self.Health` (`self.MaxHealth`))
    (if _output_developed_7
      (if _output_developed_8
        (if _output_developed_9
          (set `self.Damage` (* (`self.Damage`) 2.0))
          (else
            (set `self.Damage` (* (`self.Damage`) 1.5))))
        (else
          (set `self.Damage` (* (`self.Damage`) 1.2)))))
    (if _output_developed_5
      (if _output_developed_6
        (if _output_developed_2
          (set `self.MoveCost` (- (`self.MoveCost`) 3))
          (set `self.AttackCost` (- (`self.AttackCost`) 3))
          (set `self.JumpCost` (* (`self.MoveCost`) 3))
          (else
            (set `self.MoveCost` (- (`self.MoveCost`) 2))
            (set `self.AttackCost` (- (`self.AttackCost`) 2))))
        (else
          (set `self.MoveCost` (- (`self.MoveCost`) 1))
          (set `self.AttackCost` (- (`self.AttackCost`) 1)))))))