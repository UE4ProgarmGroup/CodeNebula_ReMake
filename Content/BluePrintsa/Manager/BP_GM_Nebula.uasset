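; BP_GM_Nebula is a game mode that registers joining players and starts a turn order.
; On PostLogin it stores each controller and its PlayerInfo, assigns the controller's PlayerIndex from the array position and updates PlayerNumber.
; If no current player is set, it makes index 0 current and calls TurnGetted on the first BP_PC_Nebula.
; Logout has no handling.
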(event `self.K2_PostLogin`
  (params (NewPlayer :type "PlayerController Object Reference"))
  (bind _asbp_pc_nebula (cast `/Game/BluePrintsa/Manager/BP_PC_Nebula` NewPlayer :!pure true))
  ;[1 1 1] Record New Player and set params about Turn and Round
  (`KismetArrayLibrary.Array_Add` (`self.AllPlayerControllers`) NewPlayer)
  (bind _returnvalue (`KismetArrayLibrary.Array_Add` (`self.PlayerInfos`) (`/Game/BluePrintsa/Manager/BP_PC_Nebula.PlayerInfo` _asbp_pc_nebula)))
  (bind _output_get (set `/Game/BluePrintsa/Manager/BP_PC_Nebula.PlayerIndex` _returnvalue _asbp_pc_nebula))
  (set `self.PlayerNumber` (+ _output_get 1))
  (if (< (`self.CurrentPlayerIndex`) 0)
    (set `self.CurrentPlayerIndex` 0)
    (bind _asbp_pc_nebula_2 (cast `/Game/BluePrintsa/Manager/BP_PC_Nebula` (`|GetArrayItem` (`self.AllPlayerControllers`))))
    (`/Game/BluePrintsa/Manager/BP_PC_Nebula.TurnGetted` _asbp_pc_nebula_2)))

(event `self.K2_OnLogout`
  (params (ExitingController :type "Controller Object Reference")))

(fn `UserConstructionScript`)