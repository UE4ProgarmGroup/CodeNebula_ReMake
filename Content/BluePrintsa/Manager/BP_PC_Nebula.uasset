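; Player controller for the turn-based Nebula game, which creates the main UI for the local player and handles turn and round flow.
; EndTurn, also on Enter for testing, runs SwitchTurn, which advances the GameMode's player index and notifies all controllers, rolling into SwitchRound after the last player.
; Gaining a turn refreshes the PlayerState and triggers each owned building's turn action.
; Comments mark a client-to-server call with client callbacks; turn-end and round-end handlers only print.
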(event `TurnEnded`
  ;[1 1 1] Switch Turn, Round - Client Handle Server Callback
  (`KismetSystemLibrary.PrintString` "Turn Ended."))

(event `RoundEnded`
  ;[1 1 1] Switch Turn, Round - Client Handle Server Callback
  (`KismetSystemLibrary.PrintString` "Round Ended."))

(event `TurnGetted`
  ;[1 1 1] Switch Turn, Round - Client Handle Server Callback
  (set `self.GetTurn` true)
  (`KismetSystemLibrary.PrintString` "Now My Turn.")
  (bind _asbp_ps_nebula (cast `/Game/BluePrintsa/Manager/BP_PS_Nebula` (`self.PlayerState`))
    (:`then`
      (`/Game/BluePrintsa/Manager/BP_PS_Nebula.Refresh` _asbp_ps_nebula)
      (for _array_element (`/Game/BluePrintsa/Manager/BP_PS_Nebula.BuildingOwned` _asbp_ps_nebula)
        (`/Game/BluePrintsa/Player/Building/BP_BuildingBase.EventActionOnTurn` _array_element)))
    (:`CastFailed`
      (`KismetSystemLibrary.PrintString` "Hello"))))

(event `SwitchTurn`
  ;[1 1 1] Switch Turn, Round - Server Callback
  ;;[1 1 1] Switch Turn /  Each Player do Settlement and Into a New Round or Next Player get Turn - Called when Player call EndTurn
  (bind _asbp_gm_nebula (cast `/Game/BluePrintsa/Manager/BP_GM_Nebula` (`GameplayStatics.GetGameMode`)))
  (bind _currentplayerindex (`/Game/BluePrintsa/Manager/BP_GM_Nebula.CurrentPlayerIndex` _asbp_gm_nebula))
  (`/Engine/EditorBlueprintResources/StandardMacros.IncrementInt` _currentplayerindex
    (:`  `
      (bind _allplayercontrollers (`/Game/BluePrintsa/Manager/BP_GM_Nebula.AllPlayerControllers` _asbp_gm_nebula))
      (for _array_element _allplayercontrollers
        (bind _asbp_pc_nebula (cast `/Game/BluePrintsa/Manager/BP_PC_Nebula` _array_element))
        (`self.TurnEnded` _asbp_pc_nebula))
      (if (>= _currentplayerindex (`/Game/BluePrintsa/Manager/BP_GM_Nebula.PlayerNumber` _asbp_gm_nebula))
        (`self.SwitchRound`)
        (else
          (bind _asbp_pc_nebula_2 (cast `/Game/BluePrintsa/Manager/BP_PC_Nebula` (`|GetArrayItem` _allplayercontrollers _currentplayerindex)))
          (`self.TurnGetted` _asbp_pc_nebula_2))))))

(event `self.ReceiveBeginPlay`
  ;[1 1 1] 创建UI
  (if (`self.IsLocalPlayerController` self)
    (bind _returnvalue (`|CreateWidget` "/Game/BluePrintsa/Widget/PlayerUI/MainUI.MainUI_C" self))
    (`UserWidget.AddToViewport` _returnvalue 0)))

(event `EndTurn`
  ;[1 1 1] Call Switch Turn - Client Call Server
  (if (`self.GetTurn`)
    (set `self.GetTurn` false)
    (`self.SwitchTurn`)
    (`KismetSystemLibrary.PrintString` "Call End Turn.")))

(event `SwitchRound`
  ;[1 1 1] Switch Turn, Round - Server Callback
  ;;[1 1 1] Into a New Round / Each Player do Settlement and First Player get Turn
  (bind _asbp_gm_nebula (cast `/Game/BluePrintsa/Manager/BP_GM_Nebula` (`GameplayStatics.GetGameMode`)))
  (bind _allplayercontrollers (`/Game/BluePrintsa/Manager/BP_GM_Nebula.AllPlayerControllers` _asbp_gm_nebula))
  (for _array_element _allplayercontrollers
    (bind _asbp_pc_nebula (cast `/Game/BluePrintsa/Manager/BP_PC_Nebula` _array_element))
    (`self.RoundEnded` _asbp_pc_nebula))
  (set `/Game/BluePrintsa/Manager/BP_GM_Nebula.CurrentPlayerIndex` 0 _asbp_gm_nebula)
  (bind _asbp_pc_nebula_2 (cast `/Game/BluePrintsa/Manager/BP_PC_Nebula` (`|GetArrayItem` _allplayercontrollers)))
  (`self.TurnGetted` _asbp_pc_nebula_2))

(event `Key|Enter`
  (params (Key :type "Key Structure"))
  ;[1 1 1] Test Turn-Base
  (:`Pressed`
    (`self.EndTurn`)))

(fn `UserConstructionScript`)