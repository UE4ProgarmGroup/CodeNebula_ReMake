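; Player camera pawn for a nebula map that also relays move, jump and attack orders to units.
; WASD axes pan it with border clamping plus a speed-scaled offset, and scrolling runs a timeline driving spring arm length and pitch.
; CamMove uses a second timeline to glide toward a star location.
; Orders branch on authority into Server or Client events, both ending in the unit's MoveMulti, JumpMulti or AttackMulti.
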(event `Move_Eve`
  (params (location :type "Vector Structure (by ref)") (MoveUnit :type "/Game/BluePrintsa/Player/Unit/BP_BaseUnit Object Reference"))
  ;[1 1 1] 移动逻辑
  (`/Engine/EditorBlueprintResources/ActorMacros.Switch Has Authority`
    (:`Authority`
      (`self.Move_Server` location MoveUnit))
    (:`Remote`
      (`self.Move_Client` location MoveUnit))))

(event `Jump_Eve`
  (params (Location :type "Vector Structure") (Unit :type "/Game/BluePrintsa/Player/Unit/BP_BaseUnit Object Reference"))
  ;[1 1 1] 跃迁逻辑
  (`/Engine/EditorBlueprintResources/ActorMacros.Switch Has Authority`
    (:`Authority`
      (`self.Jump_Server` Location Unit))
    (:`Remote`
      (`self.Jump_Client` Location Unit))))

(event `Move_Client`
  (params (location :type "Vector Structure (by ref)") (MoveUnit :type "/Game/BluePrintsa/Player/Unit/BP_BaseUnit Object Reference"))
  ;[1 1 1] 移动逻辑
  (`self.Move_Server` location MoveUnit))

(event `Jump_Client`
  (params (Location :type "Vector Structure") (Unit :type "/Game/BluePrintsa/Player/Unit/BP_BaseUnit Object Reference"))
  ;[1 1 1] 跃迁逻辑
  (`self.Jump_Server` Location Unit))

(event `Move_Server`
  (params (location :type "Vector Structure (by ref)") (MoveUnit :type "/Game/BluePrintsa/Player/Unit/BP_BaseUnit Object Reference"))
  ;[1 1 1] 移动逻辑
  (`/Game/BluePrintsa/Player/Unit/BP_BaseUnit.Move_Multi` MoveUnit location))

(event `InputAxis|MoveWS`
  (params (AxisValue :type "Float (single-precision)"))
  ;[1 1 1] WASD移动
  (`self.K2_SetActorLocation` (`KismetMathLibrary.MakeVector` (`KismetMathLibrary.FClamp` (+ AxisValue (.x (`self.K2_GetActorLocation`))) (`self.DownBorder`) (`self.UpBorder`)) (.y (`self.K2_GetActorLocation`)) (.z (`self.K2_GetActorLocation`))))
  (`self.K2_AddActorLocalOffset` (`KismetMathLibrary.MakeVector` (* (`self.CamMovSpeed`) AxisValue))))

(event `Jump_Server`
  (params (Location :type "Vector Structure") (Unit :type "/Game/BluePrintsa/Player/Unit/BP_BaseUnit Object Reference"))
  ;[1 1 1] 跃迁逻辑
  (`/Game/BluePrintsa/Player/Unit/BP_BaseUnit.Jump_Multi` Unit Location))

(event `Attack_Eve`
  (params (Attacker :type "/Game/BluePrintsa/Player/Unit/BP_BaseUnit Object Reference") (Target :type "/Game/BluePrintsa/Player/Unit/BP_BaseUnit Object Reference"))
  ;[1 1 1] 攻击逻辑
  (`/Engine/EditorBlueprintResources/ActorMacros.Switch Has Authority`
    (:`Authority`
      (`self.Attack_Server` Attacker Target))
    (:`Remote`
      (`self.Attack_Client` Attacker Target))))

(event `InputAxis|MoveAD`
  (params (AxisValue :type "Float (single-precision)"))
  ;[1 1 1] WASD移动
  (`self.K2_SetActorLocation` (`KismetMathLibrary.MakeVector` (.x (`self.K2_GetActorLocation`)) (`KismetMathLibrary.FClamp` (+ AxisValue (.y (`self.K2_GetActorLocation`))) (`self.LeftBorder`) (`self.RightBorder`)) (.z (`self.K2_GetActorLocation`))))
  (`self.K2_AddActorLocalOffset` (`KismetMathLibrary.MakeVector` 0.0 (* (`self.CamMovSpeed`) AxisValue))))

(event `Attack_Client`
  (params (Attacker :type "/Game/BluePrintsa/Player/Unit/BP_BaseUnit Object Reference") (Target :type "/Game/BluePrintsa/Player/Unit/BP_BaseUnit Object Reference"))
  ;[1 1 1] 攻击逻辑
  (`self.Attack_Server` Attacker Target))

(event `Attack_Server`
  (params (Attacker :type "/Game/BluePrintsa/Player/Unit/BP_BaseUnit Object Reference") (Target :type "/Game/BluePrintsa/Player/Unit/BP_BaseUnit Object Reference"))
  ;[1 1 1] 攻击逻辑
  (`/Game/BluePrintsa/Player/Unit/BP_BaseUnit.Attack_Multi` Attacker Target))

(event `InputAction|ScrollUp`
  (params (Key :type "Key Structure"))
  (bind _springarm (`self.SpringArm`))
  ;[1 1 1] 缩放
  (:`Pressed`
    (bind (_direction _updown _rotate) (`Timeline|时间轴_0` :!label _label)
      (:`Update`
        (`|ExecutionSequence`
          (:`then_0`
            (set `SpringArmComponent.TargetArmLength` _updown _springarm))
          (:`then_1`
            (`SceneComponent.K2_SetRelativeRotation` _springarm (`KismetMathLibrary.MakeRotator` 0.0 _rotate) false false)))))))

(event `CamMove`
  (params (StarLocation :type "Vector Structure"))
  ;[1 1 1] 平滑过渡
  (bind (_direction _time) (`Timeline|时间轴_1` :!via `PlayFromStart`)
    (:`Update`
      (`SceneComponent.K2_SetRelativeLocationAndRotation` :`self` (`self.DefaultSceneRoot`) :`NewLocation` (`KismetMathLibrary.VLerp` (`self.K2_GetActorLocation`) StarLocation _time)))))

(event `InputAction|ScrollDown`
  (params (Key :type "Key Structure"))
  ;[1 1 1] 缩放
  (:`Pressed`
    (goto _label :!via `Reverse`)))

(fn `UserConstructionScript`)