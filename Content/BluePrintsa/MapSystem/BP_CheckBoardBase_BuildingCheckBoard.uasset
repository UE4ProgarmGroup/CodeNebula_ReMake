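; Building checkerboard tile for the map system, a variant of the checkerboard base that gives itself a random appearance.
; On EventInit, Init picks a random static mesh from the Mesh array and applies it to the Planet component.
; It also sets the component's first material slot to that mesh's own default material.
; The construction script only calls the parent, and the default BeginPlay, overlap and Tick events are unused.
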(event `EventInit`
  (`self.Init`))

(fn `Init`
  (locals (NewLocalVar_0 :type "StaticMesh Object Reference"))
  (bind _planet (`self.Planet`))
  (bind _newlocalvar_0 (`local.NewLocalVar_0`))
  (set `local.NewLocalVar_0` (`KismetArrayLibrary.Array_Random` (`self.Mesh`)))
  (`StaticMeshComponent.SetStaticMesh` _planet _newlocalvar_0)
  (`PrimitiveComponent.SetMaterial` _planet 0 (`StaticMesh.GetMaterial` _newlocalvar_0 0)))

(fn `UserConstructionScript`
  (`parent.UserConstructionScript`))