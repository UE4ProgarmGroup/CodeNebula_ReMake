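; Grid tile for unit movement on a checkerboard map, tracking occupancy and serving as a click target for moves.
; At BeginPlay it caches tiles within a fixed radius as neighbours, and its box overlap registers it as the unit's board.
; It highlights free neighbours green or itself red for enemies by swapping materials.
; Right-clicking a highlighted tile has the player pawn move the selected unit, briefly disabling clicks before re-highlighting.
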(event `self.ReceiveBeginPlay`
  ;[1 1 1] 开始时获得相邻方格
  (bind _outactors (`GameplayStatics.GetAllActorsOfClass` "BP_CheckBoardBase_MovingCheckBoard_C"))
  (for _array_element _outactors
    (if (<= (`KismetMathLibrary.VSize` (- (`self.K2_GetActorLocation` _array_element) (`self.K2_GetActorLocation`))) 150.0)
      (`KismetArrayLibrary.Array_Add` (`self.Neighbours`) _array_element))))

(event `self.BoardBase.OnClicked`
  (params (TouchedComponent :type "PrimitiveComponent Object Reference") (ButtonPressed :type "Key Structure"))
  (bind _returnvalue (`GameplayStatics.GetPlayerController` 0))
  (bind _returnvalue_2 (`GameplayStatics.GetPlayerController` 0))
  (bind _asbp_pc_nebula (cast `/Game/BluePrintsa/Manager/BP_PC_Nebula` _returnvalue_2 :!pure true))
  (bind _selectedunit (`/Game/BluePrintsa/Manager/BP_PC_Nebula.SelectedUnit` _asbp_pc_nebula))
  (bind _board (`/Game/BluePrintsa/Player/Unit/BP_BaseUnit.Board` _selectedunit))
  ;[1 1 1] 右键单击简单移动
  (if (== ButtonPressed "RightMouseButton")
    (if (`self.Highlight`)
      (bind _output_get (set `/Game/BluePrintsa/Manager/BP_PC_Nebula.MoveLocation` (`self.K2_GetActorLocation`) _asbp_pc_nebula))
      (`self.Resethighlight` _board)
      (set `PlayerController.bEnableClickEvents` false _returnvalue)
      (`/Game/BluePrintsa/Manager/BP_PP_Nebula.Move_Eve` (cast `/Game/BluePrintsa/Manager/BP_PP_Nebula` (`Controller.K2_GetPawn` _returnvalue_2) :!pure true) _output_get _selectedunit)
      (`KismetSystemLibrary.Delay` 0.5)
      (set `PlayerController.bEnableClickEvents` true _returnvalue)
      (`self.SetMoveHighlight` _board)
      (else
        (`KismetSystemLibrary.PrintString` "not highlight")))))

(event `self.Box.OnComponentBeginOverlap`
  (params (OverlappedComponent :type "PrimitiveComponent Object Reference") (OtherActor :type "Actor Object Reference") (OtherComp :type "PrimitiveComponent Object Reference") (OtherBodyIndex :type Integer) (bFromSweep :type Boolean) (SweepResult :type "HitResult Structure (by ref)"))
  ;[1 1 1] 设置单位所在的方格
  (bind _asbp_base_unit (cast `/Game/BluePrintsa/Player/Unit/BP_BaseUnit` OtherActor))
  (bind _output_get (set `/Game/BluePrintsa/Player/Unit/BP_BaseUnit.Board` self _asbp_base_unit))
  (`KismetSystemLibrary.PrintString` (`/Game/BluePrintsa/MapSystem/BP_CheckBoardBase_MovingCheckBoard.name` _output_get))
  (set `self.IsOccupied` true))

(event `self.Box.OnComponentEndOverlap`
  (params (OverlappedComponent :type "PrimitiveComponent Object Reference") (OtherActor :type "Actor Object Reference") (OtherComp :type "PrimitiveComponent Object Reference") (OtherBodyIndex :type Integer))
  (set `self.IsOccupied` false))

(fn `Resethighlight`
  (bind _outactors (`GameplayStatics.GetAllActorsOfClass` "BP_CheckBoardBase_MovingCheckBoard_C"))
  (for _array_element _outactors
    (`PrimitiveComponent.SetMaterial` (`/Game/BluePrintsa/MapSystem/BP_CheckBoardBase.BoardBase` _array_element) 0 "/Game/Resource/Meterial/CheckBoard/CheckBoardMeterial.CheckBoardMeterial")
    (set `/Game/BluePrintsa/MapSystem/BP_CheckBoardBase_MovingCheckBoard.Highlight` false _array_element)
    (set `/Game/BluePrintsa/MapSystem/BP_CheckBoardBase_MovingCheckBoard.isEnermy` false _array_element)))

(fn `SetEnermyHighlight`
  (`PrimitiveComponent.SetMaterial` (`self.BoardBase`) 0 "/AnimationSharing/AnimSharingRed.AnimSharingRed")
  (set `self.isEnermy` true))

(fn `SetMoveHighlight`
  (for _array_element (`self.Neighbours`)
    (if (not (`/Game/BluePrintsa/MapSystem/BP_CheckBoardBase.IsOccupied` _array_element))
      (`PrimitiveComponent.SetMaterial` (`/Game/BluePrintsa/MapSystem/BP_CheckBoardBase.BoardBase` _array_element) 0 "/AnimationSharing/AnimSharingGreen.AnimSharingGreen")
      (set `/Game/BluePrintsa/MapSystem/BP_CheckBoardBase_MovingCheckBoard.Highlight` true _array_element))))

(fn `UserConstructionScript`
  (`parent.UserConstructionScript`))