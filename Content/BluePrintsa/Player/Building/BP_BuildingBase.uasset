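; BP_BuildingBase is the base Blueprint for player buildings, providing the resource yield a building grants when its turn action fires.
; EventActionOnTurn calls ActionOnturn, which adds the building's Material, Energy and Science to the first player's BP_PS_Nebula PlayerState.
; The same call accumulates per-round material, raises max energy by double the Energy yield, and updates lifetime scoring totals, including Works.
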(event `EventActionOnTurn`
  (`self.ActionOnturn`))

(fn `ActionOnturn`
  (bind _asbp_ps_nebula (cast `/Game/BluePrintsa/Manager/BP_PS_Nebula` (`Controller.PlayerState` (`GameplayStatics.GetPlayerController` 0)) :!pure true))
  ;[1 1 1] 统计项
  (set `/Game/BluePrintsa/Manager/BP_PS_Nebula.Material` (+ (`/Game/BluePrintsa/Manager/BP_PS_Nebula.Material` _asbp_ps_nebula) (`self.Material`)) _asbp_ps_nebula)
  (set `/Game/BluePrintsa/Manager/BP_PS_Nebula.Energy` (+ (`/Game/BluePrintsa/Manager/BP_PS_Nebula.Energy` _asbp_ps_nebula) (`self.Energy`)) _asbp_ps_nebula)
  (set `/Game/BluePrintsa/Manager/BP_PS_Nebula.SciencePoint` (+ (`self.Science`) (`/Game/BluePrintsa/Manager/BP_PS_Nebula.SciencePoint` _asbp_ps_nebula)) _asbp_ps_nebula)
  ;[1 1 1] 限制项目
  (set `/Game/BluePrintsa/Manager/BP_PS_Nebula.MaterialEveryRound` (+ (`/Game/BluePrintsa/Manager/BP_PS_Nebula.MaterialEveryRound` _asbp_ps_nebula) (`self.Material`)) _asbp_ps_nebula)
  (set `/Game/BluePrintsa/Manager/BP_PS_Nebula.MaxEnergy` (+ (`/Game/BluePrintsa/Manager/BP_PS_Nebula.MaxEnergy` _asbp_ps_nebula) (* (`self.Energy`) 2)) _asbp_ps_nebula)
  ;[1 1 1] 计分项目
  (set `/Game/BluePrintsa/Manager/BP_PS_Nebula.EnergyEverGain` (+ (`self.Energy`) (`/Game/BluePrintsa/Manager/BP_PS_Nebula.EnergyEverGain` _asbp_ps_nebula)) _asbp_ps_nebula)
  (set `/Game/BluePrintsa/Manager/BP_PS_Nebula.MaterialEverGain` (+ (`self.Material`) (`/Game/BluePrintsa/Manager/BP_PS_Nebula.MaterialEverGain` _asbp_ps_nebula)) _asbp_ps_nebula)
  (set `/Game/BluePrintsa/Manager/BP_PS_Nebula.SciencePointEverGain` (+ (`self.Science`) (`/Game/BluePrintsa/Manager/BP_PS_Nebula.SciencePointEverGain` _asbp_ps_nebula)) _asbp_ps_nebula)
  (set `/Game/BluePrintsa/Manager/BP_PS_Nebula.WorksEverGain` (+ (`self.Works`) (`/Game/BluePrintsa/Manager/BP_PS_Nebula.WorksEverGain` _asbp_ps_nebula)) _asbp_ps_nebula))

(fn `UserConstructionScript`)