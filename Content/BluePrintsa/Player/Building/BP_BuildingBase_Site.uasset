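; BP_BuildingBase_Site is a construction-site building that stands in a board slot until the real building is finished.
; Each turn action runs the parent logic, then decrements BuildLevelRemain while it is above one.
; Otherwise it spawns ClassToBuild at its own transform with the same board and slot number, writes it into the building checkboard's BuildingSlot array, and destroys itself.
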(fn `ActionOnturn`
  (bind _checkboardin (`self.CheckBoardIn`))
  (`parent.ActionOnturn`)
  (if (> (`self.BuildLevelRemain`) 1)
    (`/Engine/EditorBlueprintResources/StandardMacros.DecrementInt` (`self.BuildLevelRemain`))
    (else
      (bind _returnvalue (`|SpawnActorFromClass` (`self.ClassToBuild`) (`self.GetTransform`) "Undefined" "OverrideRootScale" null _checkboardin (`self.BuildingSlotNum`) null))
      (`KismetArrayLibrary.Array_Set` (`/Game/BluePrintsa/MapSystem/BP_CheckBoardBase_BuildingCheckBoard.BuildingSlot` (cast `/Game/BluePrintsa/MapSystem/BP_CheckBoardBase_BuildingCheckBoard` _checkboardin :!pure true)) (`self.BuildingSlotNum`) _returnvalue true)
      (`self.K2_DestroyActor`))))

(fn `UserConstructionScript`
  (`parent.UserConstructionScript`))